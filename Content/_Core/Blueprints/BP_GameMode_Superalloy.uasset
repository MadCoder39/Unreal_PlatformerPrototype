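; Game mode for Superalloy that sets display and anti-aliasing options and picks where players spawn.
; On BeginPlay it runs console commands to show the FPS counter and tune temporal AA; a tonemapper sharpen command is left unconnected.
; Its ChoosePlayerStart override returns the first BP_PlayerStart_Superalloy flagged StartHere, falling back to the last one found.
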(event `self.ReceiveBeginPlay`
  (`KismetSystemLibrary.ExecuteConsoleCommand` "stat fps" null)
  (`KismetSystemLibrary.ExecuteConsoleCommand` "r.TemporalAACurrentFrameWeight 0.08" null)
  (`KismetSystemLibrary.ExecuteConsoleCommand` "r.TemporalAASamples 2" null))

(fn `ChoosePlayerStart`
  (params (Player :type "Controller Object Reference"))
  (returns (ReturnValue :type "Actor Object Reference"))
  (locals (L_LastPlayerStart :type "/Game/_Core/Blueprints/BP_PlayerStart_Superalloy Object Reference"))
  (bind _outactors (`GameplayStatics.GetAllActorsOfClass` "/Game/_Core/Blueprints/BP_PlayerStart_Superalloy.BP_PlayerStart_Superalloy_C"))
  (for _array_element _outactors
    (bind _output_get (set `local.L_LastPlayerStart` _array_element))
    (if (`/Game/_Core/Blueprints/BP_PlayerStart_Superalloy.bStartHere` _output_get)
      (return (`local.L_LastPlayerStart`))))
  (return (`local.L_LastPlayerStart`)))

(fn `UserConstructionScript`)